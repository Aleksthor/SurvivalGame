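; Player character Blueprint that toggles the inventory and chest screens in a survival game.
; The OpenInventory action swaps the in-game UI for the inventory widget, pauses, shows the cursor, and detaches the spring arm from control rotation, restoring the saved rotation on close.
; The E key similarly toggles the chest widget while ChestOpen is set, clearing that flag on close.
; Each screen's open flag blocks the other.
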(event `Key|E` :paused true
  (params (Key :type "Key Structure"))
  (bind _ingameui (`self.inGameUI`))
  ;[1 1 1] Open Chest
  (:`Pressed`
    (if (not (`self.InventoryOpen`))
      (if (not (`GameplayStatics.IsGamePaused`))
        (`KismetSystemLibrary.DelayUntilNextTick`))
      (if (`self.bChestOpen`)
        (if (`self.ChestWidgetOpen`)
          (`GameplayStatics.SetGamePaused` false)
          (`Widget.RemoveFromParent` (stale _returnvalue))
          (set `PlayerController.bShowMouseCursor` false (`GameplayStatics.GetPlayerController` 0))
          (set `self.ChestWidgetOpen` false)
          (set `self.bChestOpen` false)
          (`UserWidget.AddToViewport` _ingameui 0)
          (else
            (bind _returnvalue (`|CreateWidget` "/Game/UI/ChestInventory_Widget.ChestInventory_Widget_C"))
            (`UserWidget.AddToViewport` _returnvalue 0)
            (`GameplayStatics.SetGamePaused` true)
            (set `PlayerController.bShowMouseCursor` true (`GameplayStatics.GetPlayerController` 0))
            (set `self.ChestWidgetOpen` true)
            (`Widget.RemoveFromParent` _ingameui)))))))

(event `InputAction|OpenInventory` :paused true
  (params (Key :type "Key Structure"))
  (bind _returnvalue (`GameplayStatics.GetPlayerController` 0))
  (bind _ingameui (`self.inGameUI`))
  (bind _springarm (`self.SpringArm`))
  (bind _returnvalue_2 (`Controller.GetControlRotation` _returnvalue))
  ;[1 1 1] Open Inventory - If open show mouse and dont move spring arm. Flip function
  (:`Pressed`
    (if (`self.ChestWidgetOpen`)
      _
      (elif (`self.InventoryOpen`)
        (`UserWidget.AddToViewport` _ingameui 0)
        (`Widget.RemoveFromParent` (stale _returnvalue_3))
        (set `PlayerController.bShowMouseCursor` false (`GameplayStatics.GetPlayerController` 0))
        (set `self.InventoryOpen` false)
        (`Controller.SetControlRotation` _returnvalue (`self.LastControlRotation`))
        (set `SpringArmComponent.bUsePawnControlRotation` true (`self.SpringArm`))
        (`GameplayStatics.SetGamePaused` false)
        (else
          (`Widget.RemoveFromParent` _ingameui)
          (bind _returnvalue_3 (`|CreateWidget` "/Game/UI/Inventory_WIdget.Inventory_WIdget_C"))
          (`UserWidget.AddToViewport` _returnvalue_3 0)
          (set `PlayerController.bShowMouseCursor` true _returnvalue)
          (set `self.InventoryOpen` true)
          (`SceneComponent.K2_SetWorldRotation` _springarm _returnvalue_2 false false)
          (set `self.LastControlRotation` _returnvalue_2)
          (set `SpringArmComponent.bUsePawnControlRotation` false _springarm)
          (`GameplayStatics.SetGamePaused` true))))))

(fn `UserConstructionScript`)